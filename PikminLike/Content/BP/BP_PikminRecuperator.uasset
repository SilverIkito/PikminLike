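; BP_PikminRecuperator is the Blueprint for a recuperator Pikmin, translating its command events into AI blackboard state.
; BeginPlay binds handlers to the follow, assault, pick-up and reset-target events.
; Each handler calls ResetBlackboard to clear the target, pick-up object and state flags on the AIRecuperatorController's blackboard.
; The follow, assault and pick-up handlers then set their own flag, leaving one state active at a time.
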(event Custom|onAddPickUp_Event_0
  (CallFunction|ResetBlackboard)
  (bind _asairecuperator_controller (Utilities|Casting|CastToAIRecuperatorController (Pawn|GetController)))
  (AI|Components|Blackboard|SetValueasBool (Variables|/Script/AIModule.AIController|GetBlackboard _asairecuperator_controller) (Variables|Default|GetkeyIsPick) true))

(event Custom|onResetTarget_Event
  (CallFunction|ResetBlackboard))

(event Custom|onAssaut_Event
  (CallFunction|ResetBlackboard)
  (bind _asairecuperator_controller (Utilities|Casting|CastToAIRecuperatorController (Pawn|GetController)))
  (AI|Components|Blackboard|SetValueasBool (Variables|/Script/AIModule.AIController|GetBlackboard _asairecuperator_controller) (Variables|Default|GetkeyIsAssaut) true))

(event Custom|onAddTargetToFollow_Event
  (CallFunction|ResetBlackboard)
  (bind _asairecuperator_controller (Utilities|Casting|CastToAIRecuperatorController (Pawn|GetController)))
  (AI|Components|Blackboard|SetValueasBool (Variables|/Script/AIModule.AIController|GetBlackboard _asairecuperator_controller) (Variables|Default|GetkeyIsFollow) true))

(event EventBeginPlay
  (EventDispatchers|AssignOnAddTargettoFollow (delegate Custom|onAddTargetToFollow_Event))
  (EventDispatchers|AssignOnResetTarget (delegate Custom|onResetTarget_Event))
  (EventDispatchers|AssignOnAssaut (delegate Custom|onAssaut_Event))
  (EventDispatchers|AssignOnAddPickUp (delegate Custom|onAddPickUp_Event_0)))

(fn ConstructionScript)

(fn ResetBlackboard
  (bind _asairecuperator_controller (Utilities|Casting|CastToAIRecuperatorController (Pawn|GetController)))
  (AI|Components|Blackboard|SetValueasObject (Variables|/Script/AIModule.AIController|GetBlackboard _asairecuperator_controller) (Variables|Default|GetkeyTarget) 0)
  (AI|Components|Blackboard|SetValueasBool (Variables|/Script/AIModule.AIController|GetBlackboard _asairecuperator_controller) (Variables|Default|GetkeyIsFollow) false)
  (AI|Components|Blackboard|SetValueasBool (Variables|/Script/AIModule.AIController|GetBlackboard _asairecuperator_controller) (Variables|Default|GetkeyIsAssaut) false)
  (AI|Components|Blackboard|SetValueasObject (Variables|/Script/AIModule.AIController|GetBlackboard _asairecuperator_controller) (Variables|Default|GetkeyObjectPickUp) 0)
  (AI|Components|Blackboard|SetValueasBool (Variables|/Script/AIModule.AIController|GetBlackboard _asairecuperator_controller) (Variables|Default|GetkeyIsPick) false))