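; BP_PikminKamikaze is a Pikmin character Blueprint that translates follow, assault and target-reset commands into AI blackboard state.
; On BeginPlay it binds to the AddTargetToFollow, Assaut and ResetTarget event dispatchers.
; Each handler clears the controller's IsFollow, IsAssaut and IsAttack keys through ResetBlackBoard, then follow or assault sets its own key.
; No kamikaze-specific logic appears here, and IsAttack is only ever cleared.
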(event Custom|onAddTargetToFollow_Event
  (CallFunction|ResetBlackBoard)
  (AI|Components|Blackboard|SetValueasBool (AI|GetBlackboard (Pawn|GetController)) (Variables|Default|GetisFollow) true))

(event Custom|onResetTarget_Event
  (CallFunction|ResetBlackBoard))

(event Custom|onAssaut_Event
  (CallFunction|ResetBlackBoard)
  (AI|Components|Blackboard|SetValueasBool (AI|GetBlackboard (Pawn|GetController)) (Variables|Default|GetisAssaut) true))

(event EventBeginPlay
  (EventDispatchers|AssignOnAddTargettoFollow (delegate Custom|onAddTargetToFollow_Event))
  (EventDispatchers|AssignOnAssaut (delegate Custom|onAssaut_Event))
  (EventDispatchers|AssignOnResetTarget (delegate Custom|onResetTarget_Event)))

(fn ConstructionScript)

(fn ResetBlackBoard
  (bind _returnvalue (Pawn|GetController))
  (bind _returnvalue_2 (AI|GetBlackboard _returnvalue))
  (AI|Components|Blackboard|SetValueasBool _returnvalue_2 (Variables|Default|GetisFollow) false)
  (AI|Components|Blackboard|SetValueasBool _returnvalue_2 (Variables|Default|GetisAssaut) false)
  (AI|Components|Blackboard|SetValueasBool _returnvalue_2 (Variables|Default|GetisAttack) false))